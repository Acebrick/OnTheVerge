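; Enemy actor that turns to face the player and can be damaged and destroyed.
; On BeginPlay it caches the player pawn, then every Tick it snaps its rotation to look from its body toward the player's capsule.
; Damage reduces Health and destroys the actor at zero, otherwise the body, head and gun meshes briefly flash a hit material before reverting.
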(event `self.ReceiveTick`
  (params (DeltaSeconds :type "Float (single-precision)"))
  (`self.FaceThePlayer`))

(event `self.ReceiveBeginPlay`
  (`self.Assign Player Ref`))

(event `self.ReceiveAnyDamage`
  (params (Damage :type "Float (single-precision)") (DamageType :type "DamageType Object Reference") (InstigatedBy :type "Controller Object Reference") (DamageCauser :type "Actor Object Reference"))
  (bind _health (`self.health`))
  (set `self.health` (- _health Damage))
  (if (<= _health 0.0)
    (`self.K2_DestroyActor`)
    (else
      (`PrimitiveComponent.SetMaterial` (`self.Body`) 0 "/Game/Materials/matEnemyHit.matEnemyHit")
      (`PrimitiveComponent.SetMaterial` (`self.Head`) 0 "/Game/Materials/matEnemyHit.matEnemyHit")
      (`PrimitiveComponent.SetMaterial` (`self.GunBody`) 0 "/Game/Materials/matEnemyHit.matEnemyHit")
      (`PrimitiveComponent.SetMaterial` (`self.GunBarrel`) 0 "/Game/Materials/matEnemyHit.matEnemyHit")
      (`KismetSystemLibrary.Delay` 0.05)
      (`PrimitiveComponent.SetMaterial` (`self.Body`) 0 "/Game/Materials/matEnemy.matEnemy")
      (`PrimitiveComponent.SetMaterial` (`self.Head`) 0 "/Game/Materials/matEnemy.matEnemy")
      (`PrimitiveComponent.SetMaterial` (`self.GunBody`) 0 "/Game/Materials/matEnemy.matEnemy")
      (`PrimitiveComponent.SetMaterial` (`self.GunBarrel`) 0 "/Game/Materials/matEnemy.matEnemy"))))

(fn `Assign Player Ref`
  (bind _asplayer (cast `/Game/Blueprints/Player` (`GameplayStatics.GetPlayerPawn` 0)))
  (set `self.playerRef` _asplayer))

(fn `FaceThePlayer`
  (`self.K2_SetActorRotation` (`KismetMathLibrary.FindLookAtRotation` (`SceneComponent.K2_GetComponentLocation` (`self.Body`)) (`SceneComponent.K2_GetComponentLocation` (`Character.CapsuleComponent` (`self.playerRef`))))))

(fn `UserConstructionScript`)