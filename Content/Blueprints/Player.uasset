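; Player character Blueprint that handles movement, jumping, mouse look and shooting through Enhanced Input.
; On BeginPlay it adds TestMappingContext to the local player's input subsystem.
; Movement follows the actor's right and forward vectors, and mouse input drives controller yaw and inverted-sign pitch.
; Shooting spawns a Bullet at BulletSpawnPos, with a CanShoot flag and FireRate delay limiting the rate of fire.
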(event `self.ReceiveBeginPlay`
  ;[1 1 1 1 90] EVENT BEGIN PLAY
  (`self.InitMappingContext`))

(event `EnhancedInput|/Game/Inputs/Shoot`
  (params (ActionValue :type Boolean) (ElapsedSeconds :type "Float (double-precision)") (TriggeredSeconds :type "Float (double-precision)") (InputAction :type "InputAction Object Reference" :default "/Game/Inputs/Shoot.Shoot"))
  ;[0 1 0.9719] Left-click, shoot the bullet
  (:`Triggered`
    (if (`self.canShoot`)
      (`self.ShootBullet`))))

(event `InitMappingContext`
  ;[0.3052 0 1] Initialise the mapping context
  (`EnhancedInputSubsystemInterface.AddMappingContext` (pcsubsystem `EnhancedInputLocalPlayerSubsystem` (`GameplayStatics.GetPlayerController` 0)) "/Game/Inputs/TestMappingContext.TestMappingContext" 0 (struct)))

(event `ShootBullet`
  ;[1 0.006409 0] Shoot the bullet
  (set `self.canShoot` false)
  (`|SpawnActorFromClass` "/Game/Blueprints/Bullet.Bullet_C" (`KismetMathLibrary.MakeTransform` (`SceneComponent.K2_GetComponentLocation` (`self.BulletSpawnPos`))) "Undefined" "MultiplyWithRoot" null null)
  (`KismetSystemLibrary.Delay` (`self.fireRate`))
  (set `self.canShoot` true))

(event `EnhancedInput|/Game/Inputs/Jump`
  (params (ActionValue :type Boolean) (ElapsedSeconds :type "Float (double-precision)") (TriggeredSeconds :type "Float (double-precision)") (InputAction :type "InputAction Object Reference" :default "/Game/Inputs/Jump.Jump"))
  ;[0 1 0.9719] Make the player jump
  (:`Triggered`
    (`self.Jump`)))

(event `EnhancedInput|/Game/Inputs/LeftAndRightMovement`
  (params (ActionValue :type "Float (double-precision)") (ElapsedSeconds :type "Float (double-precision)") (TriggeredSeconds :type "Float (double-precision)") (InputAction :type "InputAction Object Reference" :default "/Game/Inputs/LeftAndRightMovement.LeftAndRightMovement"))
  ;[0.3052 0 1] Player movement
  (:`Triggered`
    (`self.AddMovementInput` (`self.GetActorRightVector`) ActionValue)))

(event `EnhancedInput|/Game/Inputs/BackAndForwardMovement`
  (params (ActionValue :type "Float (double-precision)") (ElapsedSeconds :type "Float (double-precision)") (TriggeredSeconds :type "Float (double-precision)") (InputAction :type "InputAction Object Reference" :default "/Game/Inputs/BackAndForwardMovement.BackAndForwardMovement"))
  ;[0.3052 0 1] Player movement
  (:`Triggered`
    (`self.AddMovementInput` (`self.GetActorForwardVector`) ActionValue)))

(event `EnhancedInput|/Game/Inputs/MouseMovement`
  (params (ActionValue :type "Vector2D Structure") (ElapsedSeconds :type "Float (double-precision)") (TriggeredSeconds :type "Float (double-precision)") (InputAction :type "InputAction Object Reference" :default "/Game/Inputs/MouseMovement.MouseMovement"))
  ;[0.3052 0 1] Camera movement
  (:`Triggered`
    (`self.AddControllerYawInput` ActionValue_X)
    (`self.AddControllerPitchInput` (* ActionValue_Y -1.0))))

(fn `UserConstructionScript`)